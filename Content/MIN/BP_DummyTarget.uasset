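; BP_DummyTarget is a destructible dummy target actor that takes damage and removes itself when its health runs out.
; OnHitReact forwards the damage to a Health component and prints debug text with the remaining HP.
; When OnHpChanged reports zero or less, a DoOnce disables collision and tick, then destroys the actor through a near-instant life span.
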(event `HitReactInterface.OnHitReact`
  (params (DamageAmount :type "Float (single-precision)") (HitPoint :type "Vector Structure (by ref)") (HitNormal :type "Vector Structure (by ref)"))
  (bind _health (`self.Health`))
  (`KismetSystemLibrary.PrintString` "HIT")
  (`HealthComponent.ApplyDamage_Local` _health DamageAmount)
  (`KismetSystemLibrary.PrintString` (`KismetStringLibrary.Conv_DoubleToString` (`HealthComponent.CurrentHp` _health))))

(event `self.Health.OnHpChanged`
  (params (NewHp :type "Float (single-precision)") (Delta :type "Float (single-precision)"))
  (if (<= NewHp 0.0)
    (`/Engine/EditorBlueprintResources/StandardMacros.DoOnce` false
      (:`Completed`
        (`self.SetActorEnableCollision` false)
        (`self.SetActorTickEnabled` false)
        (`self.SetLifeSpan` 0.01)))))

(fn `UserConstructionScript`)